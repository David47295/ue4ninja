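; Paper2D player character for the ninja game mode, handling movement, jump and attack input.
; Jump and attack swap sprite flipbooks, with timers based on flipbook length for follow-up transitions; the loop transition temporarily uses the idle flipbook.
; On the local controller, Tick sets camera boom length from the distance between the first two NinjaCharacters, with a minimum.
; A helper creates the HUD, while IsMyTurn is a stub returning false.
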(event `self.ReceiveBeginPlay`)

(event `self.ReceiveTick`
  (params (DeltaSeconds :type "Float (single-precision)"))
  (bind _returnvalue (`self.GetController`))
  (`/Engine/EditorBlueprintResources/StandardMacros.IsValid` _returnvalue
    (:`Is Valid`
      (if (`Controller.IsLocalController` _returnvalue)
        (`self.SetCameraDistance`)))))

(event `InputAxis|MoveUp`
  (params (AxisValue :type "Float (single-precision)"))
  (set `self.Up` AxisValue))

(event `InputAxis|MoveRight`
  (params (AxisValue :type "Float (single-precision)"))
  (`self.MoveRight` AxisValue)
  (set `self.Right` AxisValue)
  (`self.SetIsMoving` AxisValue))

(event `InputAction|Jump`
  (params (Key :type "Key Structure"))
  (:`Pressed`
    (if (and (`self.CanJump`) (not (`self.bIsAttacking`)))
      (`self.Jump`)
      (`self.HandleJumpAnims`)))
  (:`Released`
    (`self.StopJumping`)))

(event `InputAction|Attack`
  (params (Key :type "Key Structure"))
  (:`Pressed`
    (`self.PlayAttackAnim`)
    (`self.Attack`)))

(event `Key|V`
  (params (Key :type "Key Structure")))

(event `Test`)

(event `Key|X`
  (params (Key :type "Key Structure")))

(fn `HandleJumpAnims`
  (locals (FunctionName :type String :default "JumpLoopTransition"))
  (bind _sprite (`self.Sprite`))
  (`PaperFlipbookComponent.SetFlipbook` _sprite "/Game/Sprites/Ninja/Jump/FB_NinjaJump.FB_NinjaJump")
  (`KismetSystemLibrary.K2_SetTimer` null (`local.FunctionName`) (* (`PaperFlipbookComponent.GetFlipbookLength` _sprite) 0.9)))

(fn `IsJumpAnimPlaying`
  (returns (bIsPlaying :type Boolean))
  (bind _sprite (`self.Sprite`))
  (return (and (== (`PaperFlipbookComponent.GetFlipbook` _sprite) "/Game/Sprites/Ninja/Jump/FB_NinjaJump.FB_NinjaJump") (<= (`PaperFlipbookComponent.GetPlaybackPositionInFrames` _sprite) (`PaperFlipbookComponent.GetFlipbookLengthInFrames` _sprite)))))

(fn `IsMyTurn`
  (returns (bIsMyTurn :type Boolean))
  (bind _returnvalue (`self.GetController`))
  (`/Engine/EditorBlueprintResources/StandardMacros.IsValid` _returnvalue
    (:`Is Valid`
      (cast `NinjaPlayerState` (`Controller.PlayerState` _returnvalue))
      (return false))))

(fn `JumpLoopTransition`
  ;[1 1 1] TODO: Change to Loop flipbook
  (`PaperFlipbookComponent.SetFlipbook` (`self.Sprite`) "/Game/Sprites/Ninja/Idle/FB_NinjaIdle.FB_NinjaIdle"))

(fn `PlayAttackAnim`
  (bind _sprite (`self.Sprite`))
  (`PaperFlipbookComponent.SetFlipbook` _sprite "/Game/Sprites/Ninja/GroundAttack/FB_GroundAttack.FB_GroundAttack")
  (`KismetSystemLibrary.K2_SetTimer` null "JumpLoopTransition" (`PaperFlipbookComponent.GetFlipbookLength` _sprite)))

(fn `SetCameraDistance`
  (locals (NewLocalVar_0 :type "Float (double-precision)" :default 500.0))
  (bind _newlocalvar_0 (`local.NewLocalVar_0`))
  (bind _outactors (`GameplayStatics.GetAllActorsOfClass` "/Script/Ninja.NinjaCharacter"))
  (bind _output (`|GetArrayItem` _outactors))
  (`/Engine/EditorBlueprintResources/StandardMacros.IsValid` _output
    (:`Is Valid`
      (bind _output_2 (`|GetArrayItem` _outactors 1))
      (`/Engine/EditorBlueprintResources/StandardMacros.IsValid` _output_2
        (:`Is Valid`
          (set `SpringArmComponent.TargetArmLength` (+ (`KismetMathLibrary.FMax` (* (/ (`KismetMathLibrary.VSize` (- (`self.K2_GetActorLocation` _output_2) (`self.K2_GetActorLocation` _output))) _newlocalvar_0) _newlocalvar_0) (`local.NewLocalVar_0`)) 100.0) (`self.CameraBoom`)))))))

(fn `UserConstructionScript`)