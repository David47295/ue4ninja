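; Player controller for the ninja game mode that manages the lobby, pause menu and player list UI.
; On BeginPlay it shows the lobby with UI-only input and a mouse cursor, hiding the start button on non-authority clients.
; The pause input opens a menu in the same input mode and passes it the pressed key for closing.
; The player list stays on screen only while its input is held.
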(event `self.ReceiveBeginPlay`
  (`self.Client_ShowLobby`))

(event `Client_ShowLobby`
  (bind _lobbywidget (`self.LobbyWidget`))
  (bind _returnvalue (`|CreateWidget` "/Game/Blueprints/Lobby/BP_LobbyScreen.BP_LobbyScreen_C" self))
  (set `self.LobbyWidget` _returnvalue)
  (`/Engine/EditorBlueprintResources/ActorMacros.Switch Has Authority`
    (:`Authority`
      _)
    (:`Remote`
      (`Widget.SetVisibility` (`/Game/Blueprints/Lobby/BP_LobbyScreen.StartGame_Button` _returnvalue) "Hidden")))
  (`UserWidget.AddToViewport` _lobbywidget 0)
  (`WidgetBlueprintLibrary.SetInputMode_UIOnlyEx` self _lobbywidget)
  (set `self.bShowMouseCursor` true))

(event `InputAction|Pause`
  (params (Key :type "Key Structure"))
  (:`Pressed`
    (bind _returnvalue (`|CreateWidget` "/Game/Blueprints/Huds/HudComponents/BP_PauseMenu.BP_PauseMenu_C"))
    (bind _output_get (set `self.PauseMenuWidget` _returnvalue))
    (set `/Game/Blueprints/Huds/HudComponents/BP_PauseMenu.ClosePauseScreenKey` Key _output_get)
    (`UserWidget.AddToViewport` _output_get 0)
    (`WidgetBlueprintLibrary.SetInputMode_UIOnlyEx` self (`self.PauseMenuWidget`))
    (set `self.bShowMouseCursor` true)))

(event `InputAction|OpenPlayerList`
  (params (Key :type "Key Structure"))
  (:`Pressed`
    (bind _returnvalue (`|CreateWidget` "/Game/Blueprints/Huds/HudComponents/BP_PlayerList.BP_PlayerList_C"))
    (bind _output_get (set `self.PlayerListWidget` _returnvalue))
    (`UserWidget.AddToViewport` _output_get 0))
  (:`Released`
    (`Widget.RemoveFromParent` (`self.PlayerListWidget`))))

(fn `UserConstructionScript`)