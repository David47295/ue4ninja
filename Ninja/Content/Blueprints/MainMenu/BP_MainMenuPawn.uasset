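; BP_MainMenuPawn is the main menu pawn that puts the front-end UI on screen.
; On BeginPlay it creates the BP_MainMenu widget, shows the mouse cursor and switches player 0 to UI-only input focused on that widget.
; A ShowLobbyScreen event removes all widgets and adds a new BP_LobbyScreen in their place.
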(event `self.ReceiveBeginPlay`
  (bind _returnvalue (`|CreateWidget` "/Game/Blueprints/MainMenu/BP_MainMenu.BP_MainMenu_C"))
  (bind _output_get (set `self.CurrWidget` _returnvalue))
  (`UserWidget.AddToViewport` _output_get 0)
  (set `PlayerController.bShowMouseCursor` true (`GameplayStatics.GetPlayerController` 0))
  (`WidgetBlueprintLibrary.SetInputMode_UIOnlyEx` (`GameplayStatics.GetPlayerController` 0) (`self.CurrWidget`)))

(event `ShowLobbyScreen`
  (`WidgetLayoutLibrary.RemoveAllWidgets`)
  (bind _returnvalue (`|CreateWidget` "/Game/Blueprints/Lobby/BP_LobbyScreen.BP_LobbyScreen_C"))
  (bind _output_get (set `self.LobbyWidget` _returnvalue))
  (`UserWidget.AddToViewport` _output_get 0))

(fn `UserConstructionScript`)