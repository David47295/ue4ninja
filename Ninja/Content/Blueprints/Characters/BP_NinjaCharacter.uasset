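; Playable Paper2D ninja character with jump, attack and dodge inputs and a camera that adapts to two ninjas.
; Jump animates locally and via a server event; a server event also plays the attack animation.
; Flipbook-length timers schedule follow-up animations, with the attack returning to idle through a placeholder JumpLoopTransition.
; Each tick, the camera boom length follows the distance between the first two NinjaCharacters, with a minimum.
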(event `self.ReceiveBeginPlay`)

(event `self.ReceiveTick`
  (params (DeltaSeconds :type "Float (single-precision)"))
  (`self.SetCameraDistance`))

(event `InputAction|Jump`
  (params (Key :type "Key Structure"))
  (:`Pressed`
    (`self.HandleJumpAnims`)
    (`self.Server_PlayJumpAnim`)
    (`self.Jump`))
  (:`Released`
    (`self.StopJumping`)))

(event `Server_PlayJumpAnim`
  (`self.HandleJumpAnims`))

(event `Server_PlayAtttackAnim`
  (`self.PlayAttackAnim`))

(event `InputAction|Attack`
  (params (Key :type "Key Structure"))
  (:`Pressed`
    (`self.Attack`)))

(event `InputAction|Dodge`
  (params (Key :type "Key Structure"))
  (:`Pressed`
    (`self.Dodge`)))

(event `Key|V`
  (params (Key :type "Key Structure")))

(event `Key|X`
  (params (Key :type "Key Structure")))

(fn `HandleJumpAnims`
  (locals (FunctionName :type String :default "JumpLoopTransition"))
  (bind _sprite (`self.Sprite`))
  (`PaperFlipbookComponent.SetFlipbook` _sprite (`self.JumpAnimFlipbook`))
  (`KismetSystemLibrary.K2_SetTimer` null (`local.FunctionName`) (* (`PaperFlipbookComponent.GetFlipbookLength` _sprite) 0.9)))

(fn `IsJumpAnimPlaying`
  (returns (bIsPlaying :type Boolean))
  (bind _sprite (`self.Sprite`))
  (return (and (== (`PaperFlipbookComponent.GetFlipbook` _sprite) "/Game/Sprites/Ninja/Standard/Jump/FB_NinjaJump.FB_NinjaJump") (<= (`PaperFlipbookComponent.GetPlaybackPositionInFrames` _sprite) (`PaperFlipbookComponent.GetFlipbookLengthInFrames` _sprite)))))

(fn `JumpLoopTransition`
  ;[1 1 1] TODO: Change to Loop flipbook
  (`PaperFlipbookComponent.SetFlipbook` (`self.Sprite`) (`self.IdleAnimFlipbook`)))

(fn `PlayAttackAnim`
  (bind _sprite (`self.Sprite`))
  (`PaperFlipbookComponent.SetFlipbook` _sprite "/Game/Sprites/Ninja/Standard/GroundAttack/FB_GroundAttack.FB_GroundAttack")
  (`KismetSystemLibrary.K2_SetTimer` null "JumpLoopTransition" (`PaperFlipbookComponent.GetFlipbookLength` _sprite)))

(fn `SetCameraDistance`
  (locals (NewLocalVar_0 :type "Float (double-precision)" :default 500.0))
  (bind _newlocalvar_0 (`local.NewLocalVar_0`))
  (bind _outactors (`GameplayStatics.GetAllActorsOfClass` "/Script/Ninja.NinjaCharacter"))
  (bind _output (`|GetArrayItem` _outactors))
  (`/Engine/EditorBlueprintResources/StandardMacros.IsValid` _output
    (:`Is Valid`
      (bind _output_2 (`|GetArrayItem` _outactors 1))
      (`/Engine/EditorBlueprintResources/StandardMacros.IsValid` _output_2
        (:`Is Valid`
          (set `SpringArmComponent.TargetArmLength` (+ (`KismetMathLibrary.FMax` (* (/ (`KismetMathLibrary.VSize` (- (`self.K2_GetActorLocation` _output_2) (`self.K2_GetActorLocation` _output))) _newlocalvar_0) _newlocalvar_0) (`local.NewLocalVar_0`)) 100.0) (`self.CameraBoom`)))))))

(fn `UserConstructionScript`)