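; Player-controlled 2D ninja character Blueprint with side-to-side movement, jumping and a ground attack, animated through Paper2D flipbooks.
; Tick picks walk or idle when grounded and not attacking, and rotates the sprite to face the movement direction.
; Jump and attack inputs swap flipbooks and set timers from flipbook length; JumpLoopTransition currently falls back to idle as a placeholder.
; Helper functions disable input for a timed duration and re-enable it.
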(event `self.ReceiveTick`
  (params (DeltaSeconds :type "Float (single-precision)"))
  (`self.HandleAnimation`))

(event `InputAxis|MoveRight`
  (params (AxisValue :type "Float (single-precision)"))
  (`self.MoveRight` AxisValue))

(event `InputAction|Jump`
  (params (Key :type "Key Structure"))
  (:`Pressed`
    (if (and (`self.CanJump`) (not (`self.bIsAttacking`)))
      (`self.Jump`)
      (`self.HandleJumpAnims`)))
  (:`Released`
    (`self.StopJumping`)))

(event `HandleAnimation`
  (`self.Locomotion`)
  (`self.SetSpriteDirection`))

(event `InputAction|Attack`
  (params (Key :type "Key Structure"))
  (:`Pressed`
    (`self.PlayAttackAnim`)
    (`self.Attack`)))

(event `Key|V`
  (params (Key :type "Key Structure")))

(fn `DisableMovement`
  (params (Duration :type "Float (double-precision)"))
  (locals (FunctionName :type String :default "EnableMovement"))
  (`self.DisableInput` null)
  (`KismetSystemLibrary.K2_SetTimer` null (`local.FunctionName`) Duration))

(fn `EnableMovement`
  (`self.EnableInput` null))

(fn `HandleJumpAnims`
  (locals (FunctionName :type String :default "JumpLoopTransition"))
  (bind _sprite (`self.Sprite`))
  (`PaperFlipbookComponent.SetFlipbook` _sprite "/Game/Sprites/Ninja/Jump/FB_NinjaJump.FB_NinjaJump")
  (`KismetSystemLibrary.K2_SetTimer` null (`local.FunctionName`) (* (`PaperFlipbookComponent.GetFlipbookLength` _sprite) 0.9)))

(fn `IsJumpAnimPlaying`
  (returns (bIsPlaying :type Boolean))
  (bind _sprite (`self.Sprite`))
  (return (and (== (`PaperFlipbookComponent.GetFlipbook` _sprite) "/Game/Sprites/Ninja/Jump/FB_NinjaJump.FB_NinjaJump") (<= (`PaperFlipbookComponent.GetPlaybackPositionInFrames` _sprite) (`PaperFlipbookComponent.GetFlipbookLengthInFrames` _sprite)))))

(fn `JumpLoopTransition`
  ;[1 1 1] TODO: Change to Loop flipbook
  (`PaperFlipbookComponent.SetFlipbook` (`self.Sprite`) "/Game/Sprites/Ninja/Idle/FB_NinjaIdle.FB_NinjaIdle"))

(fn `Locomotion`
  (bind _sprite (`self.Sprite`))
  (if (and (not (`NavMovementComponent.IsFalling` (`self.CharacterMovement`))) (not (`self.bIsAttacking`)))
    (if (!= (`self.GetInputAxisValue`) 0.0)
      (`PaperFlipbookComponent.SetFlipbook` _sprite "/Game/Sprites/Ninja/Walk/FB_NinjaWalk.FB_NinjaWalk")
      (else
        (`PaperFlipbookComponent.SetFlipbook` _sprite "/Game/Sprites/Ninja/Idle/FB_NinjaIdle.FB_NinjaIdle")))))

(fn `PlayAttackAnim`
  (bind _sprite (`self.Sprite`))
  (`PaperFlipbookComponent.SetFlipbook` _sprite "/Game/Sprites/Ninja/GroundAttack/FB_GroundAttack.FB_GroundAttack")
  (`KismetSystemLibrary.K2_SetTimer` null "JumpLoopTransition" (`PaperFlipbookComponent.GetFlipbookLength` _sprite)))

(fn `SetSpriteDirection`
  (bind _sprite (`self.Sprite`))
  (if (and (!= (`self.GetInputAxisValue`) 0.0) (not (`self.bIsAttacking`)))
    (if (== (`self.GetLastMovementInputVector`) (`self.GetActorRightVector`))
      (`SceneComponent.K2_SetWorldRotation` _sprite (`self.SpriteRightDir`) false false)
      (else
        (`SceneComponent.K2_SetWorldRotation` _sprite (`self.SpriteLeftDir`) false false)))))

(fn `UserConstructionScript`)