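; Game mode Blueprint for a Ninja game, holding an unfinished sketch of player turn handling.
; BeginPlay caches the controller for ActivePlayerId and casts its PlayerState to NinjaPlayerState, with nothing following the cast.
; NewFunction0 does the same for a given controller ID after a validity check.
; Logic that toggles IsMyTurn or calls BeginRound sits in disconnected nodes and never runs.
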(event `self.ReceiveBeginPlay`
  (bind _returnvalue (`GameplayStatics.GetPlayerController` (`self.ActivePlayerId`)))
  (set `self.ActivePlayerCont` _returnvalue)
  (cast `NinjaPlayerState` (`Controller.PlayerState` _returnvalue)))

(fn `NewFunction_0`
  (params (PlayerControllerID :type Integer))
  (bind _output_get (set `self.ActivePlayerCont` (`GameplayStatics.GetPlayerController` PlayerControllerID)))
  (bind _playerstate (`Controller.PlayerState` _output_get))
  (`/Engine/EditorBlueprintResources/StandardMacros.IsValid` _playerstate
    (:`Is Valid`
      (cast `NinjaPlayerState` _playerstate))))

(fn `UserConstructionScript`)